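; Moving platform Blueprint that travels toward an end point while the player character overlaps its touch trigger.
; BeginPlay caches the platform and EndPoint world locations and sets the timeline play rate from a variable.
; Overlap by a ThirdPersonCharacter plays the timeline, which lerps the platform between those locations without sweeping.
; Ending the overlap reverses the timeline, sending the platform back toward its start.
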(event OnComponentBeginOverlap(Player_Touch)
  (params (OverlappedComponent :type Primitive%20Component%20Object%20Reference) (OtherActor :type Actor%20Object%20Reference) (OtherComp :type Primitive%20Component%20Object%20Reference) (OtherBodyIndex :type Integer) (bFromSweep :type Boolean) (SweepResult :type Hit%20Result%20Structure%20%28by%20ref%29))
  (Utilities|Casting|CastToThirdPersonCharacter OtherActor)
  (bind _newtrack_0 (Timeline|Platform_Move Play)
    (:Update
      (Transformation|SetWorldLocation (Variables|Default|GetPlatform) (Math|Vector|Lerp(Vector) (Variables|Default|GetStart_Loc) (Variables|Default|GetEnd_Loc) _newtrack_0) false false))))

(event OnComponentEndOverlap(Player_Touch)
  (params (OverlappedComponent :type Primitive%20Component%20Object%20Reference) (OtherActor :type Actor%20Object%20Reference) (OtherComp :type Primitive%20Component%20Object%20Reference) (OtherBodyIndex :type Integer))
  (Utilities|Casting|CastToThirdPersonCharacter OtherActor)
  (bind _newtrack_0 (Timeline|Platform_Move Reverse)
    (:Update
      (Transformation|SetWorldLocation (Variables|Default|GetPlatform) (Math|Vector|Lerp(Vector) (Variables|Default|GetStart_Loc) (Variables|Default|GetEnd_Loc) _newtrack_0) false false))))

(event EventBeginPlay
  (Variables|Default|SetStart_Loc (Transformation|GetWorldLocation (Variables|Default|GetPlatform)))
  (Variables|Default|SetEnd_Loc (Transformation|GetWorldLocation (Variables|Default|GetEnd_Point)))
  (Components|Timeline|SetPlayRate (Variables|Default|GetPlatform_Move) (Variables|Default|GetPlayrate)))

(fn ConstructionScript)